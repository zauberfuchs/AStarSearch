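; An actor Blueprint that runs an A* pathfinding search over a generated grid when play begins.
; BeginPlay calls Search, which spawns a GridSpawner at the world origin, configures it as a small floor-tile grid and tells it to spawn.
; Search then passes that spawner and the Start and End variables to AStarSearch, whose implementation is not in these graphs.
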(event `self.ReceiveBeginPlay`
  (`self.Search`))

(fn `Search`
  (locals (NewLocalVar_0 :type "GridSpawner Object Reference"))
  (bind _returnvalue (`|SpawnActorFromClass` "/Script/AStarSearchPlugin.GridSpawner" (`KismetMathLibrary.MakeTransform` (0.0 0.0 0.0)) "Undefined" "OverrideRootScale" null null))
  (set `GridSpawner.Width` 3 _returnvalue)
  (set `GridSpawner.Height` 3 _returnvalue)
  (set `GridSpawner.Margin` 400.0 _returnvalue)
  (set `GridSpawner.Mesh` "/Game/StarterContent/Architecture/Floor_400x400.Floor_400x400" _returnvalue)
  (`GridSpawner.Spawn` _returnvalue)
  (`AStarSearchPluginBPLibrary.AStarSearch` (`self.Start`) (`self.End`) _returnvalue))

(fn `UserConstructionScript`)