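; BP_Gridspawner is a Blueprint that builds a flat grid of child actors, sized by CellsX and CellsY.
; The Construction Script calls SpawnGrid, whose nested loops add a Child Actor Component at each TargetLocation relative to the owner.
; TargetLocation steps 256 units along X per cell, then returns X to zero and steps 256 along Y per row.
; The event graph holds no active logic.
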(event `self.ReceiveBeginPlay`)

(fn `SpawnGrid`
  (bind (_targetlocation_x _targetlocation_y) (`KismetMathLibrary.BreakVector` (`self.TargetLocation`)))
  (for _ (range 1 (+ (`self.CellsY`) 1))
    (for _ (range 1 (+ (`self.CellsX`) 1))
      (`AddComponent|NODE_AddChildActorComponent-0` :`RelativeTransform` (`KismetMathLibrary.MakeTransform` (`self.TargetLocation`)))
      (set `self.TargetLocation` (+ (`self.TargetLocation`) (256.0 0.0 0.0))))
    (set `self.TargetLocation` (`KismetMathLibrary.MakeVector` 0.0 (+ _targetlocation_y 256.0)))))

(fn `UserConstructionScript`
  (`self.SpawnGrid`))